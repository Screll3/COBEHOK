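; BP_PavementGenerator is a Geometry Script generated-mesh actor that procedurally builds a short strip of pavement plates.
; On mesh rebuild it appends three PlateSize boxes in a row along X, separated by a small fixed gap.
; After each append it deletes two triangles by hard-coded index, which stay the same each pass rather than offsetting per plate.
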(event Events|EventOnRebuildGeneratedMesh
  (params (TargetMesh :type Dynamic%20Mesh%20Object%20Reference))
  (bind _platesize (Variables|Default|GetPlateSize))
  (bind _output_get (Variables|Default|SetTarget%20Mesh TargetMesh))
  (for _index (range 0 2)
    (bind _returnvalue (Class|GeometryScriptLibraryMeshPrimitiveFunctions|AppendBox :TargetMesh _output_get :Transform (Math|Transform|MakeTransform (+ (/ (Variables|Default|GetPlateSize) 2.0) (Math|Vector|MakeVector (Math|Conversions|ToFloat(Integer) (* _index (+ (.x (Variables|Default|GetPlateSize)) 5.0))) 0.0 0.0)) "0, 0, 0" "1.000000,1.000000,1.000000") :DimensionX (.x _platesize) :DimensionY (.y _platesize) :DimensionZ (.z _platesize) :Origin "Center" :Debug 0))
    (bind (_selection _returnvalue_2) (Class|GeometryScriptLibraryMeshSelectionFunctions|ConvertIndexArraytoMeshSelection _returnvalue (Utilities|Array|MakeArray 8 9) "Triangles"))
    (Class|GeometryScriptLibraryMeshBasicEditFunctions|DeleteSelectedTrianglesfromMesh _returnvalue_2 _selection false)))

(fn ConstructionScript)